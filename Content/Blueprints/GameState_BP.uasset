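; Game state Blueprint that pushes changes in shared chat messages and player data to the UI.
; The chat change event updates every ChatBox widget and calls the first player controller to refresh the host's chat.
; The player data change event refreshes the grid in top-level Bunker widgets.
; GetPlayerDataBySteamName searches the player array by unique ID, despite its name, returning a "NOTHING FOUND" placeholder on a miss.
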(event EventBeginPlay)

(event EventTick
  (params (DeltaSeconds :type Float%20%28single-precision%29)))

(event EventOnChatMessagesChanged
  ;[1 1 1] Chat replication
  ;;[1 1 1] On chat changes
  ;;;[1 1 1] Called on every client exept host
  (bind _foundwidgets (Widget|GetAllWidgetsOfClass "/Game/UI/HUD/ChatBox.ChatBox_C" false))
  (for _array_element _foundwidgets
    (Default|UpdateChat _array_element (Variables|Default|GetChatMessages)))
  ;;;[1 1 1] Updates hosts chat
  (Default|UpdateSRVChat (.AsPlayer%20Controller%20BP (Utilities|Casting|CastToPlayerController_BP (Game|GetPlayerController 0)))))

(event EventOnPlayerDataChanged
  ;[1 1 1] PlayerData
  (bind _foundwidgets (Widget|GetAllWidgetsOfClass "/Game/UI/GameUI/Bunker.Bunker_C" true))
  (for _array_element _foundwidgets
    (Default|UpdateGrid _array_element (Class|GameStateCPP|GetPlayerData))
    (Development|PrintString "Replicated array")))

(fn ConstructionScript)

(fn GetPlayerDatabySteamName
  (params (UniqueID :type String))
  (for _array_element (Variables|Default|GetPlayerDataArray)
    (if (Utilities|Enum|Equal(Enum) (.ID (Utilities|Struct|BreakPlayerData _array_element)) UniqueID)
      (return _array_element)))
  (return (Utilities|Struct|MakePlayerData "NOTHING FOUND" "Sex" 0 "" false)))