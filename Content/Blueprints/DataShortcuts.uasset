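; DataShortcuts is a set of helper getters for player and session data such as IDs, nickname and generation seeds.
; It resolves the Blueprint game state and first player controller through casts, then reads player records, local Steam ID and per-player seed from them.
; The room seed comes from the session's SessionGenSeed extra setting, returning -1 if missing or wrongly typed.
; The nickname comes from C++ user settings.
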(fn GetLocalSeedbyID
  (params (ID :type String))
  (bind _playerdata (Default|GetPlayerDatabyId (CallFunction|GetPlayerControllerBP) ID))
  (return (.LocalGenSeed (Utilities|Struct|BreakPlayerData _playerdata))))

(fn GetRoomSeed
  (bind _extrasettings (Class|AdvancedSessionsLibrary|GetSessionSettings)
    (:OnSuccess
      (bind _settingvalue (Class|AdvancedSessionsLibrary|GetSessionPropertyInt _extrasettings "SessionGenSeed")
        (:Found
          (return _settingvalue))
        (:NotFound
          (return -1))
        (:WrongType
          (return -1))))))

(fn GetGameStateBP
  (return (.AsGame%20State%20BP (Utilities|Casting|CastToGameState_BP (Class|GameStateCPP|GetGameStateCPP)))))

(fn GetPlayerControllerBP
  (return (.AsPlayer%20Controller%20BP (Utilities|Casting|CastToPlayerController_BP (Game|GetPlayerController 0)))))

(fn GetPlayerDataArray
  (return (Variables|/Script/Bunker.GameState_CPP|GetPlayerDataArray (CallFunction|GetGameStateBP))))

(fn GetPlayerNickName
  (return (Class|BunkerUserSettingsCPP|GetUserNickName (Class|BunkerUserSettingsCPP|GetBunkerUserSettingsCPP))))

(fn GetPlayerDatabyID
  (params (ID :type String))
  (bind _dataout (Class|PropertiesGeneration|GetPlayerDatabyID (CallFunction|GetGameStateBP) ID))
  (return _dataout))

(fn GetLocalPlayerID
  (return (Variables|/Game/Blueprints/PlayerController_BP.PlayerController_BP_C|GetLocalSteamID (CallFunction|GetPlayerControllerBP))))